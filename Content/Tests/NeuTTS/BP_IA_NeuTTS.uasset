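; Test Blueprint for the InoNeuTts subsystem that speaks a fixed greeting on repeat through streamed text-to-speech.
; On BeginPlay it loads the GPU-configured model, printing download progress, then activates the first bundled voice.
; Synthesized chunks append to a streaming sound wave, which starts 2D playback on first data.
; Each successful completion restarts streaming synthesis; a non-streaming SynthesizeAsync loop exists but nothing starts it.
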(event `self.ReceiveBeginPlay`
  (`InoNeuTtsSubsystem.LoadModelAsync` (subsystem `InoNeuTtsSubsystem`) (make `InoNeuTtsConfig` "nano-q4" "decoder-int8" (make `InoLlamaModelParams` 99) (make `InoLlamaContextParams` 2048 2048 2048 1 0 0 "Enabled") (make `InoOnnxSessionOptions` (`|MakeArray` "DirectMl" :!type "EInoOnnxProvider Enum"))) (delegate `CustomEvent`) (delegate `CustomEvent_3`))
  (bind _returnvalue (`StreamingSoundWave.CreateStreamingSoundWave`))
  (bind _output_get (set `self.StreamVoice` _returnvalue))
  (`ImportedSoundWave.SetInitialDesiredSampleRate` _output_get 24000)
  (`ImportedSoundWave.SetInitialDesiredNumOfChannels` _output_get 1)
  (add `ImportedSoundWave.OnPopulateAudioData` _output_get (delegate `OnPopulateAudioData_Event`)))

(event `OnPopulateAudioData_Event`
  (params (PopulatedAudioData :type "Array of Float (single-precision) (by ref)"))
  (`/Engine/EditorBlueprintResources/StandardMacros.DoOnce` false
    (:`Completed`
      (`GameplayStatics.PlaySound2D` (`self.StreamVoice`) 1.0 1.0 0.0 null null))))

(event `CustomEvent_3`
  (params (Progress :type "InoDownloadProgress Structure (by ref)"))
  (bind (_bytesreceived _totalbytes _progresspercent _currentfilename _currentfileindex _totalfiles _overallprogresspercent) (break `InoDownloadProgress` Progress))
  (`KismetSystemLibrary.PrintString` (`KismetStringLibrary.Concat_StrStr` (`KismetStringLibrary.Conv_Int64ToString` _bytesreceived) "/" (`KismetStringLibrary.Conv_Int64ToString` _totalbytes) " -------- " (`KismetStringLibrary.Conv_IntToString` _currentfileindex) "/" (`KismetStringLibrary.Conv_IntToString` _totalfiles) " ----- " (`KismetStringLibrary.Conv_DoubleToString` _overallprogresspercent)) true true (struct :`G` 0.66 :`B` 1.0 :`A` 1.0) 15.0))

(event `CustomEvent`
  (params (bSuccess :type Boolean) (ErrorMessage :type String))
  (if bSuccess
    (`KismetSystemLibrary.PrintString` "neu tts loaded")
    (bind _returnvalue (`InoNeuTtsSubsystem.ListBundledVoices` (subsystem `InoNeuTtsSubsystem`)))
    (set `self.Voice` (`|GetArrayItem` _returnvalue))
    (`InoNeuTtsSubsystem.SetActiveVoiceAsync` (subsystem `InoNeuTtsSubsystem`) (`self.Voice`) (delegate `CustomEvent_4`))))

(event `CustomEvent_4`
  (params (bSuccess :type Boolean) (ErrorMessage :type String))
  (if bSuccess
    (`KismetSystemLibrary.PrintString` "voice  loaded")
    (`InoNeuTtsSubsystem.SynthesizeStreamAsync` (subsystem `InoNeuTtsSubsystem`) "Hello there, My name is Amir" (make `InoNeuTtsOptions` 2048) 50 (delegate `CustomEvent_0`) (delegate `CustomEvent_1`) :!label _label)))

(event `CustomEvent_2`
  (params (Result :type "InoNeuTtsResult Structure (by ref)"))
  (bind (_bsuccess _errormessage _audiosamples) (break `InoNeuTtsResult` Result))
  (`StreamingSoundWave.AppendAudioDataFromRAW` (`self.StreamVoice`) _audiosamples "Int16" 24000 1)
  (`KismetSystemLibrary.PrintString` (`KismetStringLibrary.Concat_StrStr` "complete: " (`KismetStringLibrary.Conv_IntToString` (`KismetArrayLibrary.Array_Length` _audiosamples))))
  (`InoNeuTtsSubsystem.SynthesizeAsync` (subsystem `InoNeuTtsSubsystem`) "Hello there, My name is Amir" (make `InoNeuTtsOptions` 2048) (delegate `CustomEvent_2`)))

(event `CustomEvent_0`
  (params (AudioChunk :type "Array of Byte (by ref)") (bIsFinal :type Boolean))
  (`StreamingSoundWave.AppendAudioDataFromRAW` (`self.StreamVoice`) AudioChunk "Int16" 24000 1)
  (`KismetSystemLibrary.PrintString` (`KismetStringLibrary.Concat_StrStr` "chunk: " (`KismetStringLibrary.Conv_IntToString` (`KismetArrayLibrary.Array_Length` AudioChunk)))))

(event `CustomEvent_1`
  (params (Result :type "InoNeuTtsResult Structure (by ref)"))
  (if (`.bSuccess` (break `InoNeuTtsResult` Result))
    (goto _label)))

(fn `UserConstructionScript`)