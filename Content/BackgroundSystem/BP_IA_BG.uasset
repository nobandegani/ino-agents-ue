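; Layered background actor that shows five textured backdrop meshes at increasing depths, built in the construction script with no runtime logic.
; Refresh gives each layer mesh its own dynamic instance of MI_IA_BS_Backdrop and texture, then calls SetLorRotScale to place it.
; GetStartDepth derives distance along local X from layer index, pushing the last layer farther back.
; Scale grows with distance through a fixed-FOV tangent formula, keeping apparent size constant.
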(fn `GetStartDepth`
  (params (Index :type "/InoAgents/BackgroundSystem/Data/E_IA_BS_Layer Enum" :default "NewEnumerator0") (StepDepth :type "Float (double-precision)" :default 4000.0))
  (returns (Start :type "Float (single-precision)") (Depth :type "Float (single-precision)"))
  (bind _returnvalue (`KismetMathLibrary.Conv_ByteToDouble` (`KismetSystemLibrary.MakeLiteralByte` Index)))
  (bind _returnvalue_2 (+ (* StepDepth (+ _returnvalue 1.0)) 10.0))
  (return (+ (* StepDepth _returnvalue) 10.0) (select `/InoAgents/BackgroundSystem/Data/E_IA_BS_Layer` Index :`NewEnumerator0` _returnvalue_2 :`NewEnumerator1` _returnvalue_2 :`NewEnumerator2` _returnvalue_2 :`NewEnumerator3` _returnvalue_2 :`NewEnumerator4` (+ (* StepDepth (+ _returnvalue 5.0)) 10.0) :!type "Float (single-precision)")))

(fn `Refresh`
  (`|ExecutionSequence`
    (:`then_0`
      (bind _returnvalue (`KismetMaterialLibrary.CreateDynamicMaterialInstance` "/InoAgents/BackgroundSystem/Materials/MI_IA_BS_Backdrop.MI_IA_BS_Backdrop"))
      (set `self.M_Layer0` _returnvalue)
      (bind _returnvalue_2 (`KismetMaterialLibrary.CreateDynamicMaterialInstance` "/InoAgents/BackgroundSystem/Materials/MI_IA_BS_Backdrop.MI_IA_BS_Backdrop"))
      (set `self.M_Layer1` _returnvalue_2)
      (bind _returnvalue_3 (`KismetMaterialLibrary.CreateDynamicMaterialInstance` "/InoAgents/BackgroundSystem/Materials/MI_IA_BS_Backdrop.MI_IA_BS_Backdrop"))
      (set `self.M_Layer2` _returnvalue_3)
      (bind _returnvalue_4 (`KismetMaterialLibrary.CreateDynamicMaterialInstance` "/InoAgents/BackgroundSystem/Materials/MI_IA_BS_Backdrop.MI_IA_BS_Backdrop"))
      (set `self.M_Layer3` _returnvalue_4)
      (bind _returnvalue_5 (`KismetMaterialLibrary.CreateDynamicMaterialInstance` "/InoAgents/BackgroundSystem/Materials/MI_IA_BS_Backdrop.MI_IA_BS_Backdrop"))
      (set `self.M_Layer4` _returnvalue_5))
    (:`then_1`
      (`PrimitiveComponent.SetMaterial` (`self.SM_Layer0`) 0 (`self.M_Layer0`))
      (`PrimitiveComponent.SetMaterial` (`self.SM_Layer1`) 0 (`self.M_Layer1`))
      (`PrimitiveComponent.SetMaterial` (`self.SM_Layer2`) 0 (`self.M_Layer2`))
      (`PrimitiveComponent.SetMaterial` (`self.SM_Layer3`) 0 (`self.M_Layer3`))
      (`PrimitiveComponent.SetMaterial` (`self.SM_Layer4`) 0 (`self.M_Layer4`)))
    (:`then_2`
      (`MaterialInstanceDynamic.SetTextureParameterValue` (`self.M_Layer0`) "Texture" (`self.T_Layer0`))
      (`MaterialInstanceDynamic.SetTextureParameterValue` (`self.M_Layer1`) "Texture" (`self.T_Layer1`))
      (`MaterialInstanceDynamic.SetTextureParameterValue` (`self.M_Layer2`) "Texture" (`self.T_Layer2`))
      (`MaterialInstanceDynamic.SetTextureParameterValue` (`self.M_Layer3`) "Texture" (`self.T_Layer3`))
      (`MaterialInstanceDynamic.SetTextureParameterValue` (`self.M_Layer4`) "Texture" (`self.T_Layer4`)))
    (:`then_3`
      (`self.SetLorRotScale` "NewEnumerator0" (`self.SM_Layer0`))
      (`self.SetLorRotScale` "NewEnumerator1" (`self.SM_Layer1`))
      (`self.SetLorRotScale` "NewEnumerator2" (`self.SM_Layer2`))
      (`self.SetLorRotScale` "NewEnumerator3" (`self.SM_Layer3`))
      (`self.SetLorRotScale` "NewEnumerator4" (`self.SM_Layer4`)))))

(fn `SetLorRotScale`
  (params (Layer :type "/InoAgents/BackgroundSystem/Data/E_IA_BS_Layer Enum" :default "NewEnumerator0") (Target :type "SceneComponent Object Reference"))
  (bind (_start _depth) (`self.GetStartDepth` Layer))
  (bind _returnvalue (+ (`KismetSystemLibrary.MakeLiteralDouble` _start) (`KismetSystemLibrary.MakeLiteralDouble` _depth)))
  (bind _returnvalue_2 (/ (* 2.0 _returnvalue (`KismetMathLibrary.Tan` (/ 90.0 2.0))) 200.0))
  (`SceneComponent.K2_SetRelativeLocation` Target (`KismetMathLibrary.MakeVector` _returnvalue 0.0 1.0) false false)
  (`SceneComponent.SetRelativeScale3D` Target (`KismetMathLibrary.MakeVector` _returnvalue_2 _returnvalue_2 1.0))
  (`SceneComponent.K2_SetRelativeRotation` Target (struct :`Yaw` 90.0 :`Roll` 90.0) false false))

(fn `UserConstructionScript`
  (`self.Refresh`))