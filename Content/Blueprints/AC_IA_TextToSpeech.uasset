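; Agent text-to-speech component that turns streamed conversation sentences into audio for the agent's sound.
; Conversation delegates queue sentences, stripped through their first closing brace and filtered by length, plus pause marks at boundaries and completion.
; The queue runs serially through ElevenLabs, Chatterbox or NeuTTS, appending streamed chunks and advancing on completion or error.
; Pause marks, or no selected engine, append generated dithered silence instead.
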(event `TTS_Complete`
  (params (Success :type Boolean))
  (bind _sentencesqueue (`self.SentencesQueue`))
  ; Comment
  (`|ExecutionSequence`
    (:`then_0`
      (`KismetArrayLibrary.Array_Remove` (`self.SentencesQueue`)))
    (:`then_1`
      (if (`self.RunningQueue`) :!label _label
        (if (`KismetArrayLibrary.Array_IsValidIndex` _sentencesqueue)
          (if (`KismetStringLibrary.EqualEqual_StrStr` (`|GetArrayItem` _sentencesqueue) (`self.PauseMark`))
            (`StreamingSoundWave.AppendAudioDataFromRAW` (`/InoAgents/Blueprints/AC_IA_Agent.GetSoundRef` (`self.Agent Ref`)) (`InoAudioFunctionLibrary.GenerateDitheredSilence` (`/InoAgents/Blueprints/AC_IA_Agent.Default Pause Duration Ms` (`self.Agent Ref`)) 16000 1 "Int16" 0.001) "Int16" 16000 1 :!label _label_2)
            (`self.TTS_Complete` false)
            (else
              (switch `/InoAgents/Data/E_IA_TTS_Engine` (`/InoAgents/Blueprints/AC_IA_Agent.TTS` (`self.Agent Ref`))
                (:`NewEnumerator0`
                  (goto _label_2))
                (:`NewEnumerator6`
                  (`self.TTS_Elevenlabs`))
                (:`NewEnumerator7`
                  (`self.TTS_Chatterbox`))
                (:`NewEnumerator8`
                  (`self.TTS_NeuTTS`)))))
          (else
            (set `self.RunningQueue` false)
            (goto _label)))))))

(event `OnSentence_Event`
  (params (RawText :type String) (CleanText :type String))
  (bind _returnvalue (`self.Remove{}` RawText))
  ; Comment
  (if (> (`KismetStringLibrary.Len` _returnvalue) 5)
    (`KismetArrayLibrary.Array_Add` (`self.SentencesQueue`) _returnvalue)
    (if (not (`self.RunningQueue`))
      (set `self.RunningQueue` true)
      (`self.ProcessSentences`))))

(event `ProcessSentences`
  ; Comment
  (goto _label))

(event `InitDeligates`
  (`|ExecutionSequence`
    (:`then_0`
      ; Comment
      (add `InoLiteRtLmConversation.OnSentence` (`/InoAgents/Blueprints/AC_IA_Agent.GetConversationRef` (`self.Agent Ref`)) (delegate `OnSentence_Event`)))
    (:`then_1`
      ; Comment
      (add `InoLiteRtLmConversation.OnSentenceBoundary` (`/InoAgents/Blueprints/AC_IA_Agent.GetConversationRef` (`self.Agent Ref`)) (delegate `OnSentenceBoundary_Event`)))
    (:`then_2`
      ; Comment
      (add `InoLiteRtLmConversation.OnComplete` (`/InoAgents/Blueprints/AC_IA_Agent.GetConversationRef` (`self.Agent Ref`)) (delegate `OnComplete_Event`)))))

(event `OnSentenceBoundary_Event`
  ; Comment
  (`KismetArrayLibrary.Array_Add` (`self.SentencesQueue`) (`self.PauseMark`)))

(event `TTS_Elevenlabs`
  (bind _agent_ref (`self.Agent Ref`))
  (bind _soundwavestream (`/InoAgents/Blueprints/AC_IA_Agent.GetSoundRef` (`self.Agent Ref`)))
  (bind (_inputs _modelid _outputformat _languagecode _stability _seed _applytextnormalization) (break `InoElevenLabsDialogueRequest` (`/InoAgents/Blueprints/AC_IA_Agent.Elevenlabs Dialogue Config` _agent_ref)))
  ; Comment
  (bind _audiobytes (`InoElevenLabsTextToDialogueStream.StreamTextToDialogue` (make `InoElevenLabsDialogueRequest` (`|MakeArray` (make `InoElevenLabsDialogueInput` (`|GetArrayItem` (`self.SentencesQueue`)) (`/InoAgents/Blueprints/AC_IA_Agent.Elevenlabs Voice Id` _agent_ref))) _modelid _outputformat _languagecode _stability _seed _applytextnormalization))
    (:`OnAudioChunk`
      (if (or (`|EnumEquality` _outputformat "Mp3_44100_128") (`|EnumEquality` _outputformat "Mp3_44100_64") (`|EnumEquality` _outputformat "Mp3_22050_32"))
        (`StreamingSoundWave.AppendAudioDataFromEncoded` _soundwavestream _audiobytes "Mp3")
        (else
          (`StreamingSoundWave.AppendAudioDataFromRAW` _soundwavestream _audiobytes "Int16" (select `EInoElevenLabsOutputFormat` _outputformat :`Pcm_16000` 16000 :`Pcm_24000` 24000 :`Pcm_44100` 44100) 1))))
    (:`OnComplete`
      (`self.TTS_Complete` true))
    (:`OnError`
      (`self.TTS_Complete` false))))

(event `OnComplete_Event`
  (params (FullText :type String))
  ; Comment
  (`KismetArrayLibrary.Array_Add` (`self.SentencesQueue`) (`self.PauseMark`)))

(event `TTS_Chatterbox`
  ; Comment
  (`InoChatterboxTtsSubsystem.SynthesizeStreamAsync` (subsystem `InoChatterboxTtsSubsystem`) (`|GetArrayItem` (`self.SentencesQueue`)) (make `InoChatterboxVoice` "") (make `InoChatterboxSynthesisOptions` 1024) (delegate `CustomEvent_0`) (delegate `CustomEvent`) 50))

(event `CustomEvent_0`
  (params (AudioChunk :type "Array of Byte (by ref)") (bIsFinal :type Boolean) (NumGeneratedTokens :type Integer))
  ; Comment
  (`StreamingSoundWave.AppendAudioDataFromRAW` (`/InoAgents/Blueprints/AC_IA_Agent.GetSoundRef` (`self.Agent Ref`)) AudioChunk "Int16" 24000 1))

(event `CustomEvent`
  (params (bSuccess :type Boolean) (Result :type "InoChatterboxSynthesisResult Structure") (ErrorMessage :type String))
  ; Comment
  (`self.TTS_Complete` bSuccess))

(event `TTS_NeuTTS`
  (bind _returnvalue (subsystem `InoNeuTtsNanoSubsystem`))
  ; Comment
  (`InoNeuTtsNanoSubsystem.SynthesizeStreamAsync` _returnvalue (`|GetArrayItem` (`self.SentencesQueue`)) (`|GetArrayItem` (`InoNeuTtsNanoSubsystem.GetAvailableVoiceNames` _returnvalue)) (make `InoNeuTtsNanoSynthesisOptions` 2048) (delegate `CustomEvent_1`) (delegate `CustomEvent_2`)))

(event `CustomEvent_1`
  (params (AudioChunk :type "Array of Byte (by ref)") (bIsFinal :type Boolean) (NumSpeechIds :type Integer))
  ; Comment
  (`StreamingSoundWave.AppendAudioDataFromRAW` (`/InoAgents/Blueprints/AC_IA_Agent.GetSoundRef` (`self.Agent Ref`)) AudioChunk "Int16" 24000 1))

(event `CustomEvent_2`
  (params (bSuccess :type Boolean) (PcmInt16LE :type "Array of Byte (by ref)") (ErrorMessage :type String))
  ; Comment
  (`self.TTS_Complete` bSuccess))

(fn `Initialize`
  (params (AgentRef :type "/InoAgents/Blueprints/AC_IA_Agent Object Reference (by ref)"))
  (set `self.Agent Ref` AgentRef)
  (`self.InitDeligates`))

(fn `Remove{}`
  (params (Value :type String))
  (returns (ReturnValue :type String))
  (bind _returnvalue (`KismetStringLibrary.FindSubstring` Value "}"))
  (bind _returnvalue_2 (+ _returnvalue 1))
  (return (select `bool` (== _returnvalue -1) :`false` (`KismetStringLibrary.GetSubstring` (`local.Value`) _returnvalue_2 (- (`KismetStringLibrary.Len` (`local.Value`)) _returnvalue_2)) :`true` (`local.Value`))))