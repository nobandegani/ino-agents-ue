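; Demo actor that drives text-to-speech from the "Main" web UI and destroys itself, idling the engine, on Back to Menu.
; Generate requests load a hard-coded Piper model through InoTTS and synthesize the payload text asynchronously.
; Chunks feed a streaming sound wave that starts playback once on first populate; completion posts status and timings as "ttsResult".
; The Runtime TTS alternative is disconnected, and the required "engine" field selects nothing.
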(event `self.ReceiveBeginPlay`
  (`InoWebView.ShowNotification` (`InoWebUISubsystem.GetWebView` (subsystem `InoWebUISubsystem`) "Main") "TTS Started" "Info" 4.0)
  (`KismetSystemLibrary.PrintString` "TTS Started")
  (add `InoWebView.OnMessageReceived` (`InoWebUISubsystem.GetWebView` (subsystem `InoWebUISubsystem`) "Main") (delegate `OnMessageReceived_Event`))
  ; Comment
  (bind _returnvalue (`RuntimeTextToSpeech.CreateRuntimeTextToSpeech`))
  (set `self.RuntimeTTSRef` _returnvalue)
  (bind _returnvalue_2 (`StreamingSoundWave.CreateStreamingSoundWave`))
  (bind _output_get (set `self.SoundWaveStream` _returnvalue_2))
  (add `ImportedSoundWave.OnPopulateAudioState` _output_get (delegate `OnPopulateAudioState_Event`))
  (bind _returnvalue_3 (`CapturableSoundWave.CreateCapturableSoundWave`))
  (set `self.NewVar` _returnvalue_3))

(event `OnPopulateAudioState_Event`
  (`/Engine/EditorBlueprintResources/StandardMacros.DoOnce` false
    (:`Completed`
      (`GameplayStatics.PlaySound2D` (`self.SoundWaveStream`) 1.0 1.0 0.0 null null))))

(event `OnMessageReceived_Event`
  (params (Channel :type Name) (Payload :type "JsonObjectWrapper Structure (by ref)"))
  (bind _returnvalue (subsystem `InoWebUISubsystem`))
  (switch `name` Channel
    (:`backToMenu`
      ; Comment
      (`self.K2_DestroyActor`)
      (`InoWebUISubsystem.SetAutoEngineIdle` _returnvalue true)
      (`InoWebUISubsystem.SetEngineIdle` _returnvalue true))
    (:`generateTts`
      (`InoWebView.ShowNotification` (`InoWebUISubsystem.GetWebView` (subsystem `InoWebUISubsystem`) "Main") "Generate started" "Info" 4.0)
      (`KismetSystemLibrary.PrintString` "Generate started" true true (struct :`G` 0.66 :`B` 1.0 :`A` 1.0) 30.0)
      ; Comment
      (bind (_outvalue _returnvalue_2) (`|GetJsonField` Payload "engine"))
      (if _returnvalue_2
        (bind (_outvalue_2 _returnvalue_3) (`|GetJsonField` Payload "text"))
        (if _returnvalue_3
          ; Comment
          (`InoTTS.LoadModel` (subsystem `InoTTS`) (make `InoTTSModelConfig` "PiperVits" (make `InoTTSPiperConfig` "D:\\ModelsRoot\\EDIT_THIS_PATH_IN_EDITOR\\Plugins\\InoSherpa\\SherpaOnnx\\models\\vits-piper-en_US-libritts_r-medium\\en_US-libritts_r-medium.onnx" "D:\\ModelsRoot\\EDIT_THIS_PATH_IN_EDITOR\\Plugins\\InoSherpa\\SherpaOnnx\\models\\vits-piper-en_US-libritts_r-medium\\tokens.txt" "D:\\ModelsRoot\\EDIT_THIS_PATH_IN_EDITOR\\Plugins\\InoSherpa\\SherpaOnnx\\models\\vits-piper-en_US-libritts_r-medium\\espeak-ng-data")))
          (`InoTTS.SynthesizeStreamAsync` (subsystem `InoTTS`) (`KismetSystemLibrary.MakeLiteralString` _outvalue_2) (make `InoTTSOptions` 1.0) (delegate `CustomEvent`) (delegate `CustomEvent_2`)))))))

(event `CustomEvent`
  (params (AudioChunk :type "Array of Byte (by ref)") (Progress :type "Float (single-precision)") (bIsFinal :type Boolean))
  ; Comment
  (`StreamingSoundWave.AppendAudioDataFromRAW` (`self.SoundWaveStream`) AudioChunk "Int16" 22050 1))

(event `CustomEvent_0`
  (params (TextToSpeechInstance :type "RuntimeTextToSpeech Object Reference") (ChunkAudioData :type "Array of Byte (by ref)") (SampleRate :type Integer) (NumOfChannels :type Integer) (bIsFinalChunk :type Boolean))
  ; Comment
  (`StreamingSoundWave.AppendAudioDataFromRAW` (`self.SoundWaveStream`) ChunkAudioData "Float32" SampleRate NumOfChannels))

(event `CustomEvent_2`
  (params (Result :type "InoTTSResult Structure (by ref)"))
  (bind (_bsuccess _errormessage _audiosamples _samplerate _numchannels _durationseconds _generationtimeseconds) (break `InoTTSResult` Result))
  (bind _jsonobjectwrapper (make `JsonObjectWrapper`))
  ; Comment
  (`|SetJsonField` _jsonobjectwrapper "ok" _bsuccess)
  (`|SetJsonField` _jsonobjectwrapper "message" (`KismetSystemLibrary.MakeLiteralString` _errormessage))
  (`|SetJsonField` _jsonobjectwrapper "voiceDurationSec" (`KismetSystemLibrary.MakeLiteralDouble` _durationseconds))
  (`|SetJsonField` _jsonobjectwrapper "generationTimeSec" (`KismetSystemLibrary.MakeLiteralDouble` _generationtimeseconds))
  (`InoWebView.PostMessage` (`InoWebUISubsystem.GetWebView` (subsystem `InoWebUISubsystem`) "Main") "ttsResult" _jsonobjectwrapper))

(event `CustomEvent_1`
  (params (TextToSpeechInstance :type "RuntimeTextToSpeech Object Reference") (bSuccess :type Boolean) (ErrorMessage :type String))
  (bind _jsonobjectwrapper (make `JsonObjectWrapper`))
  (bind (_days _hours _minutes _seconds _milliseconds) (`KismetMathLibrary.BreakTimespan` (- (`KismetMathLibrary.UtcNow`) (struct))))
  ; Comment
  (`|SetJsonField` _jsonobjectwrapper "ok" bSuccess)
  (`|SetJsonField` _jsonobjectwrapper "message" "Error")
  (`|SetJsonField` _jsonobjectwrapper "voiceDurationSec" 0.0)
  (`|SetJsonField` _jsonobjectwrapper "generationTimeSec" (`KismetSystemLibrary.MakeLiteralDouble` (+ (`KismetMathLibrary.Conv_IntToDouble` _seconds) (/ (`KismetMathLibrary.Conv_IntToDouble` _milliseconds) 1000.0))))
  (`InoWebView.PostMessage` (`InoWebUISubsystem.GetWebView` (subsystem `InoWebUISubsystem`) "Main") "ttsResult" _jsonobjectwrapper))

(fn `UserConstructionScript`)