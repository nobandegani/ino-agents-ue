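; Actor component that runs a conversational MetaHuman agent with a LiteRT-LM language model, optional speech and mood-driven lip sync.
; It loads the LLM, then the selected TTS engine (ElevenLabs, Chatterbox Turbo or NeuTTS), then creates the conversation.
; Generated rules make replies carry emotion and audio tags, and parsed emotions set the lip-sync mood.
; Streaming sound wave PCM feeds the lip-sync generator, while status gates user messages.
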(event `OnAudioPlaybackFinished_Event`
  ; Comment
  (`self.UpdateStatus` "NewEnumerator0"))

(event `OnGeneratePCMData_Event`
  (params (PCMData :type "Array of Float (single-precision) (by ref)"))
  (bind _soundwavestream (`self.SoundWaveStream`))
  ; Comment
  (`RealisticMetaHumanLipSyncGenerator.ProcessAudioData` (`self.MoodLipSyncGenerator`) PCMData (`ImportedSoundWave.GetSampleRate` _soundwavestream) (`ImportedSoundWave.GetNumOfChannels` _soundwavestream))
  (`self.UpdateStatus` "NewEnumerator4"))

(event `OnPopulateAudioState_Event`
  (bind _soundwavestream (`self.SoundWaveStream`))
  (bind _audiocomponent (`self.AudioComponent`))
  ; Comment
  (`/Engine/EditorBlueprintResources/StandardMacros.DoOnce` false
    (:`Completed`
      (`ImportedSoundWave.SetNumSamplesPerChunk` _soundwavestream (/ (`ImportedSoundWave.GetSampleRate` _soundwavestream) 100))
      (`AudioComponent.SetSound` _audiocomponent (`self.SoundWaveStream`))
      (`AudioComponent.Play` _audiocomponent 0.0))))

(event `InitializeInternally`
  (bind _moodlipsyncgenerator (`self.MoodLipSyncGenerator`))
  (`|ExecutionSequence`
    (:`then_0`
      ; Comment
      (bind _returnvalue (`|AddComponentByClass` :`self` (`self.GetOwner`) :`Class` "/Script/Engine.AudioComponent" :`bManualAttachment` true))
      (set `self.AudioComponent` _returnvalue)
      (`SceneComponent.K2_AttachToComponent` (`self.AudioComponent`) (`Actor.RootComponent` (`self.GetOwner`)) "None" "SnapToTarget" "SnapToTarget" "KeepRelative" true))
    (:`then_1`
      ; Comment
      (bind _returnvalue_2 (`StreamingSoundWave.CreateStreamingSoundWave`))
      (set `self.SoundWaveStream` _returnvalue_2)
      (add `ImportedSoundWave.OnPopulateAudioState` (`self.SoundWaveStream`) (delegate `OnPopulateAudioState_Event`))
      (add `ImportedSoundWave.OnGeneratePCMData` (`self.SoundWaveStream`) (delegate `OnGeneratePCMData_Event`))
      (add `ImportedSoundWave.OnAudioPlaybackFinished` (`self.SoundWaveStream`) (delegate `OnAudioPlaybackFinished_Event`)))
    (:`then_2`
      ; Comment
      (bind _returnvalue_3 (`|AddComponentByClass` (`self.GetOwner`) "/InoAgents/Blueprints/AC_IA_TextToSpeech.AC_IA_TextToSpeech_C"))
      (set `self.TextToSpeech` _returnvalue_3))
    (:`then_3`
      ; Comment
      (bind _returnvalue_4 (`RealisticMetaHumanLipSyncGenerator.CreateRealisticMetaHumanLipSyncWithMoodGenerator` (`self.Lipsync Configuration`) :!label _label))
      (set `self.MoodLipSyncGenerator` _returnvalue_4)
      (`RealisticMetaHumanLipSyncGenerator.SetMood` _moodlipsyncgenerator "Neutral")
      (`RealisticMetaHumanLipSyncGenerator.SetMoodIntensity` _moodlipsyncgenerator 0.5))
    (:`then_4`
      (goto _label))
    (:`then_5`
      (if (`self.Use Default UI`)
        (bind _returnvalue_5 (`|AddComponentByClass` (`self.GetOwner`) "/InoAgents/Blueprints/AC_IA_UI.AC_IA_UI_C"))
        (`/InoAgents/Blueprints/AC_IA_UI.Init` _returnvalue_5 self)))))

(event `SetupChatterboxTurbo`
  (bind _returnvalue (enumliteral `EInoChatterboxTurboNativeVariant` "Q4F16"))
  (bind _returnvalue_2 (subsystem `InoChatterboxTurboNativeSubsystem`))
  ; Comment
  (if (`InoChatterboxTurboNativeSubsystem.IsModelDownloaded` _returnvalue_2 _returnvalue)
    (`self.On_Model_Update` "Loading TTS")
    (else
      (`self.On_Model_Update` "Downloading TTS")))
  (`InoChatterboxTurboNativeSubsystem.LoadModelsAsync` _returnvalue_2 (make `InoChatterboxTurboNativeModelConfig` _returnvalue false "Q4F16" "Q4F16" "Q4F16" "Q4F16" (make `InoChatterboxTurboNativePerformanceOptions` 0 1 false false false)) (delegate `On_Chatterbox_Download_Progress`) (delegate `On_Chatterbox_Model_Loaded`)))

(event `StartModelPrep`
  (bind _returnvalue (subsystem `InoLiteRtLmSubsystem`))
  (bind _llm_config (`self.LLM_Config`))
  (bind _llm_model_name (`self.LLM_Model_Name`))
  ; Comment
  (`self.SetUpRules`)
  (setmembers `InoLiteRtLmModelConfig` :`StructRef` _llm_config :`ModelFileName` _llm_model_name :`Backend` (`self.LLM_Backend`) :`SystemMessage` (`KismetStringLibrary.Concat_StrStr` (`self.Rules`) " \n" (`self.Personality`)) :`ActivationType` (`self.LLM_ActivationType`))
  (if (`InoLiteRtLmSubsystem.IsModelDownloaded` _returnvalue _llm_model_name)
    (`self.On_Model_Update` "Loading LLM")
    (else
      (`self.On_Model_Update` "Downloading LLM")))
  (`InoLiteRtLmSubsystem.LoadModelAsync` _returnvalue _llm_config (delegate `On_LiteRT_Download_Progress`) (delegate `On_LiteRT_Model_Loaded`)))

(event `On_LiteRT_Download_Progress`
  (params (Progress :type "InoDownloadProgress Structure (by ref)"))
  (bind (_bytesreceived _totalbytes _progresspercent _currentfilename _currentfileindex _totalfiles _overallprogresspercent) (break `InoDownloadProgress` Progress))
  ; Comment
  (`self.On_Model_Download` (== _overallprogresspercent 100.0) "Downloading LLM" _overallprogresspercent (`KismetMathLibrary.Conv_Int64ToInt` (/ _bytesreceived 1000000)) (`KismetMathLibrary.Conv_Int64ToInt` (/ _totalbytes 1000000))))

(event `On_Chatterbox_Download_Progress`
  (params (Percent :type "Float (single-precision)") (BytesReceived :type Integer64) (TotalBytes :type Integer64) (bCompleted :type Boolean))
  ; Comment
  (`self.On_Model_Download` bCompleted "Downloading TTS" Percent (`KismetMathLibrary.Conv_Int64ToInt` (/ BytesReceived 1000000)) (`KismetMathLibrary.Conv_Int64ToInt` (/ TotalBytes 1000000))))

(event `On_LiteRT_Model_Loaded`
  (params (bSuccess :type Boolean) (ErrorMessage :type String))
  ; Comment
  (if bSuccess
    (`self.On_Model_Update` "Loading TTS")
    (switch `/InoAgents/Data/E_IA_TTS_Engine` (`self.TTS`)
      (:`NewEnumerator0`
        (`self.On_TTS_Loaded` true))
      (:`NewEnumerator6`
        (`self.On_TTS_Loaded` true))
      (:`NewEnumerator7`
        (`self.SetupChatterboxTurbo`))
      (:`NewEnumerator8`
        (`self.SetupNeuTTSNano` :!label _label_2))
      (:`NewEnumerator9`
        (goto _label_2)))))

(event `On_Chatterbox_Model_Loaded`
  (params (bSuccess :type Boolean) (ErrorMessage :type String))
  ; Comment
  (`self.On_TTS_Loaded` bSuccess ErrorMessage))

(event `self.ReceiveEndPlay`
  (params (EndPlayReason :type "EEndPlayReason Enum" :default "Destroyed"))
  (bind _returnvalue (subsystem `InoChatterboxTurboNativeSubsystem`))
  (bind _returnvalue_2 (subsystem `InoLiteRtLmSubsystem`))
  (bind _returnvalue_3 (subsystem `InoNeuTtsSubsystem`))
  ; Comment
  (`|ExecutionSequence`
    (:`then_0`
      (if (`InoLiteRtLmSubsystem.IsModelLoaded` _returnvalue_2)
        (`InoLiteRtLmSubsystem.UnloadModel` _returnvalue_2)))
    (:`then_1`
      (if (`InoChatterboxTurboNativeSubsystem.IsModelsLoaded` _returnvalue)
        (`InoChatterboxTurboNativeSubsystem.UnloadModels` _returnvalue)))
    (:`then_2`
      (if (`InoNeuTtsSubsystem.IsModelLoaded` _returnvalue_3)
        (`InoNeuTtsSubsystem.UnloadModel` _returnvalue_3)))))

(event `SetupNeuTTSNano`
  (bind _returnvalue (subsystem `InoNeuTtsSubsystem`))
  (bind _inoneuttsconfig (make `InoNeuTtsConfig` (select `bool` (`|EnumEquality` (`self.TTS`) "NewEnumerator8") :`false` "air-q4" :`true` "nano-q4") "decoder-int8" (make `InoLlamaModelParams` (select `EInoLiteRtLmBackend` (`self.TTS_Backend`) :`Gpu` 99)) (make `InoLlamaContextParams` 2048 2048 512 1 0 0 "Auto" true false "Q4_0" "Q4_0") (make `InoOnnxSessionOptions` (`|MakeArray` "Cpu" :!type "EInoOnnxProvider Enum"))))
  ; Comment
  (if (`InoNeuTtsSubsystem.IsModelDownloaded` _returnvalue _inoneuttsconfig)
    (`self.On_Model_Update` "Loading TTS")
    (else
      (`self.On_Model_Update` "Downloading TTS")))
  (`InoNeuTtsSubsystem.LoadModelAsync` _returnvalue _inoneuttsconfig (delegate `CustomEvent`) (delegate `CustomEvent_0`)))

(event `On_TTS_Loaded`
  (params (Success :type Boolean) (ErrMessage :type String))
  (bind _soundwavestream (`self.SoundWaveStream`))
  ; Comment
  (if Success
    (if (not (`|EnumEquality` (`self.TTS`) "NewEnumerator0"))
      (`ImportedSoundWave.SetInitialDesiredSampleRate` _soundwavestream (select `/InoAgents/Data/E_IA_TTS_Engine` (`self.TTS`) :`NewEnumerator6` (select `EInoElevenLabsOutputFormat` (`.OutputFormat` (break `InoElevenLabsDialogueRequest` (`self.Elevenlabs Dialogue Config`))) :`Mp3_44100_128` 44100 :`Mp3_44100_64` 44100 :`Mp3_22050_32` 22050 :`Pcm_16000` 16000 :`Pcm_24000` 24000 :`Pcm_44100` 44100 :`Ulaw_8000` 8000) :`NewEnumerator7` (`InoChatterboxTurboNativeSubsystem.GetOutputSampleRate` (subsystem `InoChatterboxTurboNativeSubsystem`)) :`NewEnumerator8` (`InoNeuTtsSubsystem.GetSampleRate` (subsystem `InoNeuTtsSubsystem`))))
      (`ImportedSoundWave.SetInitialDesiredNumOfChannels` _soundwavestream 1))
    (`self.On_Model_Update` "Loading model")
    (`self.CustomEvent_2`)))

(event `CustomEvent_0`
  (params (Progress :type "InoDownloadProgress Structure (by ref)"))
  (bind (_bytesreceived _totalbytes _progresspercent _currentfilename _currentfileindex _totalfiles _overallprogresspercent) (break `InoDownloadProgress` Progress))
  ; Comment
  (`self.On_Model_Download` (== _overallprogresspercent 100.0) "Downloading TTS" _overallprogresspercent (`KismetMathLibrary.Conv_Int64ToInt` (/ _bytesreceived 1000000)) (`KismetMathLibrary.Conv_Int64ToInt` (/ _totalbytes 1000000))))

(event `CustomEvent`
  (params (bSuccess :type Boolean) (ErrorMessage :type String))
  (bind _returnvalue (subsystem `InoNeuTtsSubsystem`))
  ; Comment
  (if bSuccess
    (bind _returnvalue_2 (`InoNeuTtsSubsystem.ListBundledVoices` _returnvalue))
    (`InoNeuTtsSubsystem.SetActiveVoiceAsync` _returnvalue (`|GetArrayItem` _returnvalue_2) (delegate `CustomEvent_1`))
    (else
      (`self.On_TTS_Loaded` bSuccess ErrorMessage))))

(event `CustomEvent_2`
  (bind _conversation (`self.Conversation`))
  ; Comment
  (bind _returnvalue (`InoLiteRtLmSubsystem.CreateConversation` (subsystem `InoLiteRtLmSubsystem`)))
  (set `self.Conversation` _returnvalue)
  (`InoLiteRtLmConversation.SetSentenceSplitFlags` _conversation 27)
  (`InoLiteRtLmConversation.SetTagStripFlags` _conversation 5)
  (`InoLiteRtLmConversation.SetUserContext` _conversation "user name" (`self.Player Name`))
  (`/InoAgents/Blueprints/AC_IA_TextToSpeech.Initialize` (`self.TextToSpeech`) self)
  (`self.SetConvoDeligates`)
  (`self.SetInternalDeligates`)
  (`InoWebView.PostMessage` (`InoWebUISubsystem.GetWebView` (subsystem `InoWebUISubsystem`) "Main") "showChat" (make `JsonObjectWrapper`))
  (`KismetSystemLibrary.Delay` 0.2)
  (`self.UpdateStatus` "NewEnumerator0"))

(event `CustomEvent_1`
  (params (bSuccess :type Boolean) (ErrorMessage :type String))
  ; Comment
  (`self.On_TTS_Loaded` bSuccess ErrorMessage))

(event `SetConvoDeligates`
  (bind _conversation (`self.Conversation`))
  ; Comment
  (add `InoLiteRtLmConversation.OnSentence` _conversation (delegate `OnSentence_Event_0`))
  (add `InoLiteRtLmConversation.OnToken` _conversation (delegate `CustomEvent_3`))
  (add `InoLiteRtLmConversation.OnComplete` _conversation (delegate `CustomEvent_4`))
  (add `InoLiteRtLmConversation.OnUserMessage` _conversation (delegate `CustomEvent_5`)))

(event `CustomEvent_5`
  (params (UserText :type String))
  ; Comment
  (`self.On_User_Message` UserText))

(event `OnSentence_Event_0`
  (params (RawText :type String) (CleanText :type String))
  ; Comment
  (bind (_success _returnvalue) (`self.GetEmotionFromToken` RawText))
  (if _success
    (`self.UpdateEmotionFromString` _returnvalue)))

(event `CustomEvent_3`
  (params (RawText :type String) (CleanText :type String))
  ; Comment
  (`self.On_Conversation_Token` RawText CleanText))

(event `CustomEvent_4`
  (params (FullText :type String))
  ; Comment
  (`self.On_Conversation_Complete` FullText))

(event `SetInternalDeligates`
  ; Comment
  (add `self.On_Emotion_Changed` (delegate `On_Emotion_Changed_Event`)))

(event `On_Emotion_Changed_Event` :!signature `self.On_Emotion_Changed`
  (params (`New Emotion` :type "ERealisticMetaHumanLipSyncMood Enum" :default "Neutral") (`Old Emotion` :type "ERealisticMetaHumanLipSyncMood Enum" :default "Neutral"))
  ; Comment
  (`RealisticMetaHumanLipSyncGenerator.SetMood` (`self.MoodLipSyncGenerator`) `New Emotion`))

(fn `CanSendMessage`
  (returns (Return :type Boolean))
  (return (`|EnumEquality` (`self.Status`) "NewEnumerator0")))

(fn `GetAudioRef`
  (returns (AudioComponent :type "AudioComponent Object Reference"))
  (return (`self.AudioComponent`)))

(fn `GetConversationRef`
  (returns (Conversation :type "InoLiteRtLmConversation Object Reference"))
  (return (`self.Conversation`)))

(fn `GetEmotionFromToken`
  (params (Value :type String))
  (returns (Success :type Boolean) (ReturnValue :type String))
  (bind _returnvalue (`KismetStringLibrary.FindSubstring` Value "}"))
  (bind _returnvalue_2 (`KismetStringLibrary.FindSubstring` Value "{"))
  (bind _returnvalue_3 (+ _returnvalue_2 1))
  (return (and (!= _returnvalue_2 -1) (!= _returnvalue -1)) (`KismetStringLibrary.GetSubstring` (`local.Value`) _returnvalue_3 (- _returnvalue _returnvalue_3))))

(fn `GetLipsyncMoodComponent`
  (returns (MoodLipSyncGenerator :type "RealisticMetaHumanLipSyncGenerator Object Reference"))
  (return (`self.MoodLipSyncGenerator`)))

(fn `GetModelOptions`
  (returns (LLM_Model_Options :type "Array of String") (LLM_Backend_Options_Autoset :type "Array of String") (LLM_Activation_Options_AutoSet :type "Array of String") (TTS_Model_Options_AutoSet :type "Array of String") (TTS_Backend_Options_Autoset :type "Array of String") (TTS_Activation_Options_AutoSet :type "Array of String"))
  (return (`self.LLM_Model_Options`) (`self.LLM_Backend_Options_Autoset`) (`self.LLM_Activation_Options_AutoSet`) (`self.TTS_Model_Options_AutoSet`) (`self.TTS_Backend_Options_Autoset`) (`self.TTS_Activation_Options_AutoSet`)))

(fn `GetSoundRef`
  (returns (SoundWaveStream :type "StreamingSoundWave Object Reference"))
  (return (`self.SoundWaveStream`)))

(fn `Initialize`
  (params (DefaultVoiceId :type String) (Personality :type String) (UseDefaultUI :type Boolean))
  (set `self.Elevenlabs Voice Id` DefaultVoiceId)
  (set `self.Personality` Personality)
  (set `self.Use Default UI` UseDefaultUI)
  (`self.SetDefaultOptionsAutoset`)
  (`self.InitializeInternally`))

(fn `SendUserMessage`
  (params (UserText :type String))
  (bind _return (`self.CanSendMessage`))
  (if _return
    (`InoLiteRtLmConversation.SendMessageAsync` (`self.Conversation`) UserText)
    (`self.UpdateStatus` "NewEnumerator2")))

(fn `SetDefaultOptionsAutoset`
  (bind _tts_model_options_autoset (`self.TTS_Model_Options_AutoSet`))
  (bind _emotion_options_autoset (`self.Emotion_Options_AutoSet`))
  (`|ExecutionSequence`
    (:`then_0`
      (`KismetArrayLibrary.Array_Clear` (`self.LLM_Backend_Options_Autoset`))
      (`KismetArrayLibrary.Array_Clear` (`self.TTS_Backend_Options_Autoset`))
      (for _array_element (`|MakeArray` "Cpu" "Gpu" "Npu" :!type "EInoLiteRtLmBackend Enum")
        (bind _returnvalue (`|GetEnumeratorNameAsString` _array_element))
        (`KismetArrayLibrary.Array_Add` (`self.LLM_Backend_Options_Autoset`) _returnvalue)
        (`KismetArrayLibrary.Array_Add` (`self.TTS_Backend_Options_Autoset`) _returnvalue)))
    (:`then_1`
      (`KismetArrayLibrary.Array_Clear` (`self.LLM_Activation_Options_AutoSet`))
      (`KismetArrayLibrary.Array_Clear` (`self.TTS_Activation_Options_AutoSet`))
      (for _array_element_2 (`|MakeArray` "F32" "F16" "I16" "I8" :!type "EInoLiteRtLmActivationType Enum")
        (bind _returnvalue_2 (`|GetEnumeratorNameAsString` _array_element_2))
        (`KismetArrayLibrary.Array_Add` (`self.LLM_Activation_Options_AutoSet`) _returnvalue_2)
        (`KismetArrayLibrary.Array_Add` (`self.TTS_Activation_Options_AutoSet`) _returnvalue_2)))
    (:`then_2`
      (`KismetArrayLibrary.Array_Clear` _tts_model_options_autoset)
      (for _array_element_3 (`|MakeArray` "NewEnumerator0" "NewEnumerator6" "NewEnumerator7" "NewEnumerator8" :!type "/InoAgents/Data/E_IA_TTS_Engine Enum")
        (`KismetArrayLibrary.Array_Add` _tts_model_options_autoset (`|GetEnumeratorNameAsString` _array_element_3))))
    (:`then_3`
      (`KismetArrayLibrary.Array_Clear` _emotion_options_autoset)
      (for _array_element_4 (`|MakeArray` "Neutral" "Happiness" "Sadness" "Disgust" "Anger" "Surprise" "Fear" "Confidence" "Excitement" "Boredom" "Playfulness" "Confusion" :!type "ERealisticMetaHumanLipSyncMood Enum")
        (`KismetArrayLibrary.Array_Add` _emotion_options_autoset (`|GetEnumeratorNameAsString` _array_element_4))))))

(fn `SetModelOptions`
  (params (LLM_Model_Name :type String) (LLM_Backend :type "String (by ref)") (LLM_Activation :type "String (by ref)") (TTS_Model_Name :type "String (by ref)") (TTS_Backend :type "String (by ref)") (TTS_Activation :type "String (by ref)") (`Player Name` :type String))
  (`|ExecutionSequence`
    (:`then_0`
      (set `self.LLM_Model_Name` LLM_Model_Name)
      (set `self.LLM_Backend` (cast `EInoLiteRtLmBackend` (`KismetMathLibrary.Conv_IntToByte` (`KismetArrayLibrary.Array_Find` (`self.LLM_Backend_Options_Autoset`) LLM_Backend))))
      (set `self.LLM_ActivationType` (cast `EInoLiteRtLmActivationType` (`KismetMathLibrary.Conv_IntToByte` (`KismetArrayLibrary.Array_Find` (`self.LLM_Activation_Options_AutoSet`) LLM_Activation)))))
    (:`then_1`
      (set `self.TTS` (cast `/InoAgents/Data/E_IA_TTS_Engine` (`KismetMathLibrary.Conv_IntToByte` (`KismetArrayLibrary.Array_Find` (`self.TTS_Model_Options_AutoSet`) TTS_Model_Name))))
      (set `self.TTS_Backend` (cast `EInoLiteRtLmBackend` (`KismetMathLibrary.Conv_IntToByte` (`KismetArrayLibrary.Array_Find` (`self.TTS_Backend_Options_Autoset`) TTS_Backend))))
      (set `self.TTS_ActivationType` (cast `EInoLiteRtLmActivationType` (`KismetMathLibrary.Conv_IntToByte` (`KismetArrayLibrary.Array_Find` (`self.TTS_Activation_Options_AutoSet`) TTS_Activation)))))
    (:`then_2`
      (set `self.Player Name` `Player Name`))))

(fn `SetUpRules`
  (locals (EmotionRule :type String) (AudioTagsRule :type String))
  (bind _array (`|MakeArray`))
  (bind _emotion_options_autoset (`self.Emotion_Options_AutoSet`))
  (bind _tts (`self.TTS`))
  (bind _returnvalue (select `/InoAgents/Data/E_IA_TTS_Engine` (`self.TTS`) :`NewEnumerator0` _array :`NewEnumerator6` (`self.AudioTags_Elevenlabs_Options`) :`NewEnumerator7` (`self.AudioTags_Chatterbox_Options`) :`NewEnumerator8` _array))
  (set `local.EmotionRule` "Start every response with your current emotion in curly braces, choosing from:")
  (for (_array_element _array_index) _emotion_options_autoset
    (set `local.EmotionRule` (`KismetStringLibrary.Concat_StrStr` (`local.EmotionRule`) " " (`KismetStringLibrary.Concat_StrStr` "{" _array_element "}") (select `bool` (== _array_index (`KismetArrayLibrary.Array_LastIndex` _emotion_options_autoset)) :`false` "," :`true` "."))))
  (if (or (`|EnumEquality` _tts "NewEnumerator6") (`|EnumEquality` _tts "NewEnumerator7"))
    (set `local.AudioTagsRule` "Add expressive TTS tags in square brackets throughout your speech where delivery shifts. Place tags at the start of a line or before any phrase where the delivery changes. Use tags naturally — not every sentence needs one, but shift emotions when the conversation calls for it. Only use tags from the list below, written exactly as shown:")
    (for (_array_element_2 _array_index_2) _returnvalue
      (set `local.AudioTagsRule` (`KismetStringLibrary.Concat_StrStr` (`local.AudioTagsRule`) " " (`KismetStringLibrary.Concat_StrStr` "[" _array_element_2 "]") (select `bool` (== _array_index_2 (`KismetArrayLibrary.Array_LastIndex` _returnvalue)) :`false` "," :`true` ".")))))
  (set `self.Rules` (`KismetStringLibrary.Concat_StrStr` "RULES: \n" "Keep responses to 2-4 lines of plain text, no markdown or emojis. \n" (`local.EmotionRule`) " \n" (`local.AudioTagsRule`) " \n")))

(fn `UpdateEmotionFromString`
  (params (EmotionStr :type String))
  (returns (Emotion :type "ERealisticMetaHumanLipSyncMood Enum"))
  (locals (InputEmotion :type "ERealisticMetaHumanLipSyncMood Enum" :default "Neutral") (Old_Emotion :type "ERealisticMetaHumanLipSyncMood Enum" :default "Neutral"))
  (bind _emotion_options_autoset (`self.Emotion_Options_AutoSet`))
  (bind _returnvalue (`KismetArrayLibrary.Array_Find` _emotion_options_autoset (`local.EmotionStr`)))
  (`|ExecutionSequence`
    (:`then_0`
      (`KismetSystemLibrary.PrintString` (`KismetStringLibrary.Concat_StrStr` "Emotion: input ->" (`local.EmotionStr`)) true false (struct :`R` 0.030758 :`B` 1.0 :`A` 1.0) 30.0))
    (:`then_1`
      (if (== _returnvalue -1)
        (`KismetSystemLibrary.PrintString` (`KismetStringLibrary.Concat_StrStr` "Emotion: failed to parse ->" (`local.EmotionStr`)) true false (struct :`R` 1.0 :`G` 0.042312 :`B` 0.137499 :`A` 1.0) 30.0)
        (set `local.InputEmotion` (`self.Emotion`))
        (else
          (bind _output_get (set `local.InputEmotion` (cast `ERealisticMetaHumanLipSyncMood` (`KismetMathLibrary.Conv_IntToByte` _returnvalue))))
          (`KismetSystemLibrary.PrintString` (`KismetStringLibrary.Concat_StrStr` "Emotion: valid-> " (`|GetArrayItem` _emotion_options_autoset _returnvalue) " -- " (`|GetEnumeratorNameAsString` _output_get)) true false (struct :`R` 1.0 :`G` 0.453285 :`A` 1.0) 30.0))))
    (:`then_2`
      (if (not (`|EnumEquality` (`self.Emotion`) (`local.InputEmotion`)))
        (set `local.Old_Emotion` (`self.Emotion`))
        (set `self.Emotion` (`local.InputEmotion`))
        (`self.On_Emotion_Changed` (`self.Emotion`) (`local.Old_Emotion`)))
      (return (`local.InputEmotion`)))))

(fn `UpdateStatus`
  (params (InStatus :type "/InoAgents/Data/E_IA_AgentStatus Enum" :default "NewEnumerator0"))
  (if (not (`|EnumEquality` InStatus (`self.Status`)))
    (set `self.Status` InStatus)
    (`self.On_Status_Changed` (`self.Status`))))