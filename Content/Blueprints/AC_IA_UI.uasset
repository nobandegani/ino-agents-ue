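; Bridge component between an AI agent and a web-based UI for configuring and chatting with the agent in a demo.
; On Init it binds agent events, pushing emotion, status, send availability and streamed chat tokens as JSON channel messages, and posts default model options.
; Incoming web messages apply LLM/TTS options and start model prep, send user text, or reopen the menu level.
; Loading and download-progress helpers exist but are unwired.
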(event `Init`
  (params (Agent :type "/InoAgents/Blueprints/AC_IA_Agent Object Reference"))
  (bind _agent (`self.Agent`))
  (bind _agent_2 (`self.Agent`))
  (bind _agent_3 (`self.Agent`))
  (set `self.Agent` Agent)
  (add `/InoAgents/Blueprints/AC_IA_Agent.On_Model_Update` _agent (delegate `On_LLM_Update_Event`))
  (add `/InoAgents/Blueprints/AC_IA_Agent.On_Model_Download` _agent (delegate `On_LLM_Download_Event`))
  (add `/InoAgents/Blueprints/AC_IA_Agent.On_Emotion_Changed` _agent_2 (delegate `On_Emotion_Changed_Event`))
  (add `/InoAgents/Blueprints/AC_IA_Agent.On_Status_Changed` _agent_2 (delegate `On_Status_Changed_Event`))
  (add `/InoAgents/Blueprints/AC_IA_Agent.On_Conversation_Token` _agent_3 (delegate `On_Conversation_Token_Event`))
  (add `/InoAgents/Blueprints/AC_IA_Agent.On_Conversation_Complete` _agent_3 (delegate `On_Conversation_Complete_Event`))
  (add `/InoAgents/Blueprints/AC_IA_Agent.On_User_Message` _agent_3 (delegate `On_User_Message_Event`))
  (add `InoWebView.OnMessageReceived` (`self.GetWebView`) (delegate `OnMessageReceived_Event`))
  (bind _jsonobjectwrapper (`self.GetDefaultOptionsPayload`))
  (`InoWebView.PostMessage` (`self.GetWebView`) "showAgentConfig" _jsonobjectwrapper))

(event `On_LLM_Update_Event`
  (params (Status :type String))
  (`KismetSystemLibrary.PrintString` Status true true (struct :`G` 0.66 :`B` 1.0 :`A` 1.0) 50.0))

(event `On_LLM_Download_Event`
  (params (Complete :type Boolean) (Status :type String) (Percent :type "Float (double-precision)") (Recieved :type Integer) (Total :type Integer)))

(event `On_Emotion_Changed_Event`
  (params (`New Emotion` :type "ERealisticMetaHumanLipSyncMood Enum" :default "Neutral") (`Old Emotion` :type "ERealisticMetaHumanLipSyncMood Enum" :default "Neutral"))
  (`self.setEmotion` (`KismetStringLibrary.ToLower` (`|GetEnumeratorNameAsString` `New Emotion`))))

(event `On_User_Message_Event`
  (params (Text :type String))
  (`self.chatMessage` true Text true))

(event `On_Status_Changed_Event`
  (params (Status :type "/InoAgents/Data/E_IA_AgentStatus Enum" :default "NewEnumerator0"))
  (`self.setStatus` (`|GetEnumeratorNameAsString` Status))
  (bind _return (`/InoAgents/Blueprints/AC_IA_Agent.CanSendMessage` (`self.Agent`)))
  (`self.setChatCanSend` _return))

(event `On_Conversation_Token_Event`
  (params (Raw :type String) (Clean :type String))
  (`self.chatMessage` false Clean))

(event `On_Conversation_Complete_Event`
  (params (Text :type String))
  (`self.chatMessage` false "" true))

(event `OnMessageReceived_Event`
  (params (Channel :type Name) (Payload :type "JsonObjectWrapper Structure (by ref)"))
  (set `self.TempOnMessagePayload` Payload)
  (switch `name` Channel
    (:`startDemo`
      (`self.OnStartDemo`))
    (:`sendChatMessage`
      (bind (_outvalue _returnvalue) (`|GetJsonField` (`self.TempOnMessagePayload`) "text"))
      (if _returnvalue
        (`/InoAgents/Blueprints/AC_IA_Agent.SendUserMessage` (`self.Agent`) _outvalue)))
    (:`backToMenu`
      (`GameplayStatics.OpenLevelBySoftObjectPtr` "/Game/Maps/L_IAD_Default.L_IAD_Default"))))

(fn `chatMessage`
  (params (`IsUser?` :type Boolean) (text :type String) (complete :type Boolean))
  (returns (Channel :type Name) (JsonObjectWrapper :type "JsonObjectWrapper Structure"))
  (bind _jsonobjectwrapper (make `JsonObjectWrapper`))
  (`|SetJsonField` _jsonobjectwrapper "role" (`KismetSystemLibrary.MakeLiteralString` (select `bool` `IsUser?` :`false` "ai" :`true` "user")))
  (`|SetJsonField` _jsonobjectwrapper "text" text)
  (`|SetJsonField` _jsonobjectwrapper "complete" complete)
  (`InoWebView.PostMessage` (`self.GetWebView`) "chatMessage" _jsonobjectwrapper)
  (return "chatMessage" _jsonobjectwrapper))

(fn `DownloadProgressPage`
  (params (Show :type Boolean) (Message :type String :default "Downloading model") (Percent :type "Float (double-precision)") (recieved :type Integer) (total :type Integer))
  (returns (JsonObjectWrapper :type "JsonObjectWrapper Structure"))
  (bind _jsonobjectwrapper (make `JsonObjectWrapper`))
  (`|SetJsonField` _jsonobjectwrapper "percent" Percent)
  (`|SetJsonField` _jsonobjectwrapper "receivedMB" recieved)
  (`|SetJsonField` _jsonobjectwrapper "totalMB" total)
  (if Show
    (`|SetJsonField` _jsonobjectwrapper "message" Message))
  (`InoWebView.PostMessage` (`self.GetWebView`) (select `bool` Show :`false` "updateDownloadProgress" :`true` "showDownloadProgress" :!type "Name") _jsonobjectwrapper)
  (return _jsonobjectwrapper))

(fn `GetDefaultOptionsPayload`
  (returns (JsonObjectWrapper :type "JsonObjectWrapper Structure"))
  (bind _jsonobjectwrapper (make `JsonObjectWrapper`))
  (bind _jsonobjectwrapper_2 (make `JsonObjectWrapper`))
  (bind _jsonobjectwrapper_3 (make `JsonObjectWrapper`))
  (bind _agent (`self.Agent`))
  (bind (_llm_model_options _llm_backend_options_autoset _llm_activation_options_autoset _tts_model_options_autoset _tts_backend_options_autoset _tts_activation_options_autoset) (`/InoAgents/Blueprints/AC_IA_Agent.GetModelOptions` _agent))
  (`|SetJsonField` _jsonobjectwrapper_2 "playerName" (`/InoAgents/Blueprints/AC_IA_Agent.Player Name` _agent))
  (`|SetJsonField` _jsonobjectwrapper_2 "llmModel" (`|GetArrayItem` _llm_model_options))
  (`|SetJsonField` _jsonobjectwrapper_2 "llmBackend" (`|GetArrayItem` _llm_backend_options_autoset))
  (`|SetJsonField` _jsonobjectwrapper_2 "llmActivation" (`|GetArrayItem` _llm_activation_options_autoset))
  (`|SetJsonField` _jsonobjectwrapper_2 "ttsModel" (`|GetArrayItem` _tts_model_options_autoset))
  (`|SetJsonField` _jsonobjectwrapper_2 "ttsBackend" (`|GetArrayItem` _tts_backend_options_autoset))
  (`|SetJsonField` _jsonobjectwrapper_2 "ttsActivation" (`|GetArrayItem` _tts_activation_options_autoset))
  (`|SetJsonField` _jsonobjectwrapper_3 "llmModels" _llm_model_options)
  (`|SetJsonField` _jsonobjectwrapper_3 "llmBackends" _llm_backend_options_autoset)
  (`|SetJsonField` _jsonobjectwrapper_3 "llmActivations" _llm_activation_options_autoset)
  (`|SetJsonField` _jsonobjectwrapper_3 "ttsModels" _tts_model_options_autoset)
  (`|SetJsonField` _jsonobjectwrapper_3 "ttsBackends" _tts_backend_options_autoset)
  (`|SetJsonField` _jsonobjectwrapper_3 "ttsActivations" _tts_activation_options_autoset)
  (`|SetJsonField` _jsonobjectwrapper "agent" "test")
  (`|SetJsonField` _jsonobjectwrapper "defaults" _jsonobjectwrapper_2)
  (`|SetJsonField` _jsonobjectwrapper "options" _jsonobjectwrapper_3)
  (return _jsonobjectwrapper))

(fn `GetWebView`
  (returns (ReturnValue :type "InoWebView Object Reference"))
  (return (`InoWebUISubsystem.GetWebView` (subsystem `InoWebUISubsystem`) (`self.Name`))))

(fn `OnStartDemo`
  (bind _agent (`self.Agent`))
  (bind _temponmessagepayload (`self.TempOnMessagePayload`))
  (bind _temponmessagepayload_2 (`self.TempOnMessagePayload`))
  (bind _outvalue (`|GetJsonField` _temponmessagepayload "llmModel"))
  (bind _outvalue_2 (`|GetJsonField` _temponmessagepayload "llmBackend"))
  (bind _outvalue_3 (`|GetJsonField` _temponmessagepayload "llmActivation"))
  (bind _outvalue_4 (`|GetJsonField` _temponmessagepayload_2 "ttsModel"))
  (bind _outvalue_5 (`|GetJsonField` _temponmessagepayload_2 "ttsBackend"))
  (bind _outvalue_6 (`|GetJsonField` _temponmessagepayload_2 "ttsActivation"))
  (bind _outvalue_7 (`|GetJsonField` (`self.TempOnMessagePayload`) "playerName"))
  (`/InoAgents/Blueprints/AC_IA_Agent.SetModelOptions` _agent (`KismetSystemLibrary.MakeLiteralString` _outvalue) (`KismetSystemLibrary.MakeLiteralString` _outvalue_2) (`KismetSystemLibrary.MakeLiteralString` _outvalue_3) (`KismetSystemLibrary.MakeLiteralString` _outvalue_4) (`KismetSystemLibrary.MakeLiteralString` _outvalue_5) (`KismetSystemLibrary.MakeLiteralString` _outvalue_6) (`KismetSystemLibrary.MakeLiteralString` _outvalue_7))
  (`/InoAgents/Blueprints/AC_IA_Agent.StartModelPrep` _agent))

(fn `setChatCanSend`
  (params (CanSend :type Boolean))
  (returns (Channel :type Name) (JsonObjectWrapper :type "JsonObjectWrapper Structure"))
  (bind _jsonobjectwrapper (make `JsonObjectWrapper`))
  (`|SetJsonField` _jsonobjectwrapper "canSend" CanSend)
  (`InoWebView.PostMessage` (`self.GetWebView`) "setChatCanSend" _jsonobjectwrapper)
  (return "setChatCanSend" _jsonobjectwrapper))

(fn `setEmotion`
  (params (emotion :type String))
  (returns (Channel :type Name) (JsonObjectWrapper :type "JsonObjectWrapper Structure"))
  (bind _jsonobjectwrapper (make `JsonObjectWrapper`))
  (`|SetJsonField` _jsonobjectwrapper "emotion" emotion)
  (`InoWebView.PostMessage` (`self.GetWebView`) "setEmotion" _jsonobjectwrapper)
  (return "setEmotion" _jsonobjectwrapper))

(fn `setStatus`
  (params (status :type String))
  (returns (Channel :type Name) (JsonObjectWrapper :type "JsonObjectWrapper Structure"))
  (bind _jsonobjectwrapper (make `JsonObjectWrapper`))
  (`|SetJsonField` _jsonobjectwrapper "status" status)
  (`InoWebView.PostMessage` (`self.GetWebView`) "setStatus" _jsonobjectwrapper)
  (return "setStatus" _jsonobjectwrapper))

(fn `showLoading`
  (params (Message :type String :default "Loading model"))
  (returns (ReturnValue :type Name) (JsonObjectWrapper :type "JsonObjectWrapper Structure"))
  (bind _jsonobjectwrapper (make `JsonObjectWrapper`))
  (`|SetJsonField` _jsonobjectwrapper "message" Message)
  (`InoWebView.PostMessage` (`self.GetWebView`) "showLoading" _jsonobjectwrapper)
  (return "showLoading" _jsonobjectwrapper))